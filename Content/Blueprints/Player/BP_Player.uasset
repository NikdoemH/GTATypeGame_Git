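; Player character Blueprint for a third-person shooter, handling movement, camera look, rifle equip, aiming and firing through Enhanced Input.
; Equip toggles rifle visibility after a short delay, while an aim timeline blends spring arm length and offset, with further zoom available while aiming.
; Holding shoot with the rifle equipped loops a timer that plays the fire montage, whose notify runs a debug-drawn muzzle line trace without processing hits.
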(event Custom|Shoot%20Rifle
  (bind _rifle (Variables|Default|GetRifle))
  (bind _returnvalue (Transformation|GetSocketTransform _rifle "Muzzle" "RTS_World"))
  (Animation|Montage|PlayMontage (Variables|Character|GetMesh) "/Game/Animation/Rifle/Fire_Rifle_Montage.Fire_Rifle_Montage"
    (:OnNotifyBegin
      (Collision|MultiLineTraceByChannel (.location _returnvalue) (+ (.location _returnvalue) (* (Math|Vector|GetForwardVector (.rotation _returnvalue)) 5e+03)) "TraceTypeQuery1" false 0 "ForDuration"))))

(event Input|EnhancedActionEvents|EnhancedInputActionIA_Move
  (params (ActionValue :type Vector%202D%20Structure) (ElapsedSeconds :type Float%20%28double-precision%29) (TriggeredSeconds :type Float%20%28double-precision%29) (InputAction :type Input%20Action%20Object%20Reference :default "/Game/Input/Player/Input/IA_Move.IA_Move"))
  (bind _returnvalue (Pawn|GetControlRotation :!class /Script/Engine.Pawn))
  (bind _returnvalue_2 (Pawn|GetControlRotation :!class /Script/Engine.Pawn))
  (Pawn|Input|AddMovementInput (Math|Vector|GetRightVector (Math|Rotator|MakeRotator (.roll _returnvalue) 0.0 (.yaw _returnvalue))) (.x ActionValue) false)
  (Pawn|Input|AddMovementInput (Math|Vector|GetForwardVector (Math|Rotator|MakeRotator (.roll _returnvalue_2) 0.0 (.yaw _returnvalue_2))) (.y ActionValue) false))

(event Input|EnhancedActionEvents|EnhancedInputActionIA_Camera
  (params (ActionValue :type Vector%202D%20Structure) (ElapsedSeconds :type Float%20%28double-precision%29) (TriggeredSeconds :type Float%20%28double-precision%29) (InputAction :type Input%20Action%20Object%20Reference :default "/Game/Input/Player/Input/IA_Camera.IA_Camera"))
  (Pawn|Input|AddControllerYawInput (.x ActionValue))
  (Pawn|Input|AddControllerPitchInput (* (.y ActionValue) -1.0)))

(event Input|EnhancedActionEvents|EnhancedInputActionIA_EquipRifle
  (params (ActionValue :type Boolean) (ElapsedSeconds :type Float%20%28double-precision%29) (TriggeredSeconds :type Float%20%28double-precision%29) (InputAction :type Input%20Action%20Object%20Reference :default "/Game/Input/Player/Input/IA_EquipRifle.IA_EquipRifle"))
  ;[1 1 1] Equip Gun
  (:Started
    (bind _isa (Utilities|FlowControl|FlipFlop)
      (:A
        _)
      (:B
        _))
    (bind _output_get (Variables|Default|SetRifleEquipped _isa))
    (if _output_get
      (Utilities|FlowControl|Delay 0.5)
      (Rendering|SetVisibility (Variables|Default|GetRifle) true false)
      (else
        (Utilities|FlowControl|Delay 0.5)
        (Rendering|SetVisibility (Variables|Default|GetRifle) false false)))))

(event Input|EnhancedActionEvents|EnhancedInputActionIA_AimWeapon
  (params (ActionValue :type Boolean) (ElapsedSeconds :type Float%20%28double-precision%29) (TriggeredSeconds :type Float%20%28double-precision%29) (InputAction :type Input%20Action%20Object%20Reference :default "/Game/Input/Player/Input/IA_AimWeapon.IA_AimWeapon"))
  (bind _springarm (Variables|Default|GetSpringArm))
  (:Started
    (Variables|Default|SetIsAming true)
    (bind _armlenght (Timeline|Aim Play)
      (:Update
        (Variables|/Script/Engine.SpringArmComponent|SetTargetArmLength _springarm (Math|Float|Lerp 4.5e+02 1e+02 _armlenght))
        (Variables|/Script/Engine.SpringArmComponent|SetSocketOffset _springarm (Math|Vector|MakeVector (Math|Float|Lerp 0.0 5e+01 _armlenght) (.y (Variables|/Script/Engine.SpringArmComponent|GetSocketOffset _springarm)) (Math|Float|Lerp 0.0 5e+01 _armlenght))))))
  (:Completed
    (Variables|Default|SetIsAming false)
    (Timeline|Aim Reverse)))

(event Input|EnhancedActionEvents|EnhancedInputActionIA_Shoot
  (params (ActionValue :type Boolean) (ElapsedSeconds :type Float%20%28double-precision%29) (TriggeredSeconds :type Float%20%28double-precision%29) (InputAction :type Input%20Action%20Object%20Reference :default "/Game/Input/Player/Input/IA_Shoot.IA_Shoot"))
  (:Started
    (if (Variables|Default|GetRifleEquipped)
      (bind _returnvalue (Utilities|Time|SetTimerbyEvent (delegate Custom|Shoot%20Rifle) 0.1 true))))
  (:Completed
    (Utilities|Time|ClearandInvalidateTimerbyHandle _returnvalue)))

(event Input|EnhancedActionEvents|EnhancedInputActionIA_Zoom
  (params (ActionValue :type Boolean) (ElapsedSeconds :type Float%20%28double-precision%29) (TriggeredSeconds :type Float%20%28double-precision%29) (InputAction :type Input%20Action%20Object%20Reference :default "/Game/Input/Player/Input/IA_Zoom.IA_Zoom"))
  (:Triggered
    (if (Variables|Default|GetIsAming)
      (Variables|/Script/Engine.SpringArmComponent|SetTargetArmLength (Variables|Default|GetSpringArm) -5e+01))))

(event EventBeginPlay
  (Input|AddMappingContext (PlayerController|LocalPlayerSubsystems|GetEnhancedInputLocalPlayerSubsystem (Game|GetPlayerController 0)) "/Game/Input/Player/IMC_Player.IMC_Player" 0 "(bIgnoreAllPressedKeysUntilRelease=True,bForceImmediately=False,bNotifyUserSettings=False)"))

(fn ConstructionScript)